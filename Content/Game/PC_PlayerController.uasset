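; Player controller that handles input for the pause menu and for dummy victory and defeat screens used in testing.
; The pause input, ignored on the "Main" level, creates or reuses a cached PauseMenu widget, shows it and pauses the game.
; The two test inputs each create their screen, then share one AddToViewport node targeting both widgets and set the game to unpaused.
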(event `InputAction|OpenPauseMenu`
  (params (Key :type "Key Structure"))
  ;[1 1 1] Pause Menu
  ;
  ; On pause menu button press, create a pause menu widget, add to viewport and pause the game.
  (:`Pressed`
    (bind _returnvalue (`GameplayStatics.GetCurrentLevelName` true))
    (if (`KismetStringLibrary.NotEqual_StrStr` _returnvalue "Main")
      (`/Engine/EditorBlueprintResources/StandardMacros.IsValid` (`self.PauseMenuReference`)
        (:`Is Valid`
          _)
        (:`Is Not Valid`
          (bind _returnvalue_2 (`|CreateWidget` "/Game/UI/PauseMenu.PauseMenu_C"))
          (set `self.PauseMenuReference` _returnvalue_2)))
      (`UserWidget.AddToViewport` (`self.PauseMenuReference`) 0)
      (`GameplayStatics.SetGamePaused` true))))

(event `InputAction|DummyVictoryCondition`
  (params (Key :type "Key Structure"))
  ;[1 1 1] Dummy Victory/Loss Buttons
  ;
  ; Simulate game over conditions for testing
  (:`Pressed`
    (bind _returnvalue (`|CreateWidget` "/Game/UI/VictoryScreen.VictoryScreen_C"))
    (`UserWidget.AddToViewport` (stale `InputAction|DummyDefeatCondition` _returnvalue) 0 :!label _label)
    (`UserWidget.AddToViewport` _returnvalue 0)
    (`GameplayStatics.SetGamePaused` false)))

(event `InputAction|DummyDefeatCondition`
  (params (Key :type "Key Structure"))
  ;[1 1 1] Dummy Victory/Loss Buttons
  ;
  ; Simulate game over conditions for testing
  (:`Pressed`
    (bind _returnvalue (`|CreateWidget` "/Game/UI/DefeatScreen.DefeatScreen_C"))
    (goto _label)))

(fn `UserConstructionScript`)